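; Valve actor for what appears to be a valve puzzle, spinning its Vanasm component while another actor overlaps it.
; Overlap start enables input and plays a timeline, and overlap end disables input and stops it.
; Each timeline update adds a local rotation combining the track's pitch with the BeginPlay world rotation, then sends NewFunctionMessage to the player controller.
; The Rotate function is an empty stub.
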(event `self.ReceiveBeginPlay`
  (set `self.NewVar` (`SceneComponent.K2_GetComponentRotation` (`self.vanasm`))))

(event `self.ReceiveActorBeginOverlap`
  (params (OtherActor :type "Actor Object Reference"))
  (`self.EnableInput` null)
  (bind (_direction _newtrack_0) (`Timeline|Timeline` :!label _label)
    (:`Update`
      (`SceneComponent.K2_AddLocalRotation` (`self.vanasm`) (`KismetMathLibrary.ComposeRotators` (`KismetMathLibrary.MakeRotator` 0.0 _newtrack_0) (`self.NewVar`)) false false)
      (message `/Game/vanabulmacası/vanaçevirme.NewFunction` (`GameplayStatics.GetPlayerController` 0)))))

(event `self.ReceiveActorEndOverlap`
  (params (OtherActor :type "Actor Object Reference"))
  (`self.DisableInput` null)
  (goto _label :!via `Stop`))

(fn `rotate`)

(fn `UserConstructionScript`)