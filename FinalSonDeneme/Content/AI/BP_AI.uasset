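; BP_AI is an enemy character that chases the player and triggers a game-over jumpscare on contact.
; Pawn sensing sets a SeeingPlayer blackboard flag, and a retriggerable delay clears it shortly after sightings stop.
; Capsule overlap with the player disables input, plays a scream sound, lights a spotlight, blends the view to itself and loops a ghost animation, then opens the main menu.
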(event `self.PS_AI_Sense.OnSeePawn`
  (params (Pawn :type "Pawn Object Reference"))
  ;[1 1 1] Chase Player
  (cast `/Game/ThirdPerson/Blueprints/BP_ThirdPersonCharacter` Pawn)
  (`BlackboardComponent.SetValueAsBool` (`AIBlueprintHelperLibrary.GetBlackboard` (`AIBlueprintHelperLibrary.GetAIController` self)) "SeeingPlayer" true)
  (`KismetSystemLibrary.RetriggerableDelay` 0.6)
  (`BlackboardComponent.SetValueAsBool` (`AIBlueprintHelperLibrary.GetBlackboard` (`AIBlueprintHelperLibrary.GetAIController` self)) "SeeingPlayer" false))

(event `self.Capsule.OnComponentBeginOverlap`
  (params (OverlappedComponent :type "PrimitiveComponent Object Reference") (OtherActor :type "Actor Object Reference") (OtherComp :type "PrimitiveComponent Object Reference") (OtherBodyIndex :type Integer) (bFromSweep :type Boolean) (SweepResult :type "HitResult Structure (by ref)"))
  (if (== OtherActor (`GameplayStatics.GetPlayerCharacter` 0))
    (`self.StartJumpscare`)))

(event `StartJumpscare`
  (`self.DisableInput` (`GameplayStatics.GetPlayerController` 0))
  (`GameplayStatics.PlaySound2D` "/Game/AI/KisaltCiglikdeneme.KisaltCiglikdeneme" 1.0 1.0 0.0 null null)
  (`SceneComponent.SetVisibility` (`self.SpotLight`) true false)
  (`PlayerController.SetViewTargetWithBlend` (`GameplayStatics.GetPlayerController` 0) self 0.0 "VTBlend_Linear" 0.0 false)
  (`SkeletalMeshComponent.PlayAnimation` (`self.Mesh`) "/Game/blueprint/ghost/GhostDaughter_Anim.GhostDaughter_Anim" true)
  (`KismetSystemLibrary.Delay` 2.0)
  (`GameplayStatics.OpenLevelBySoftObjectPtr` "/Game/MainMenuLevel.MainMenuLevel"))

(fn `UserConstructionScript`)